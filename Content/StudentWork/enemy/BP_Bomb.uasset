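; BP_Bomb is an explosive actor that, once damaged, flashes and then explodes.
; The construction script creates a dynamic instance of M_bombFlash on the static mesh.
; The first AnyDamage event, gated by DoOnce, plays a timeline that drives the material's flashTimer parameter.
; When the timeline finishes, the bomb applies radial damage around its mesh and destroys itself.
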(event `self.ReceiveAnyDamage`
  (params (Damage :type "Float (single-precision)") (DamageType :type "DamageType Object Reference") (InstigatedBy :type "Controller Object Reference") (DamageCauser :type "Actor Object Reference"))
  (`/Engine/EditorBlueprintResources/StandardMacros.DoOnce` false
    (:`Completed`
      (bind (_direction _newtrack_0) (`Timeline|flash`)
        (:`Update`
          (`MaterialInstanceDynamic.SetScalarParameterValue` (`self.FlashMat`) "flashTimer" _newtrack_0))
        (:`Finished`
          (`GameplayStatics.ApplyRadialDamage` :`BaseDamage` 50.0 :`Origin` (`SceneComponent.K2_GetComponentLocation` (`self.StaticMesh`)) :`DamageRadius` 500.0 :`DamageCauser` self :`InstigatedByController` null)
          (`self.K2_DestroyActor`))))))

(fn `UserConstructionScript`
  (bind _returnvalue (`PrimitiveComponent.CreateDynamicMaterialInstance` (`self.StaticMesh`) 0 "/Game/StudentWork/enemy/M_bombFlash.M_bombFlash" "None"))
  (set `self.FlashMat` _returnvalue))