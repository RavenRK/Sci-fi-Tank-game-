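; Enemy turret Blueprint, apparently a randomly firing mobile variant, that shoots six projectiles per fire event.
; BeginPlay runs the parent logic, then overrides the BaseStates stat struct.
; FireEvent calls FireProj once at each of six arrow components, using that arrow's world transform and the shared projectile class, size and damage.
; The file shows no movement or fire-timing logic of its own.
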(event `self.ReceiveBeginPlay`
  (`parent.ReceiveBeginPlay`)
  (bind _output_get (set `self.BaseStates` (make `/Game/StudentWork/enemy/S_TurretBaseStates` 350.0 350.0 1000.0 1.0 0.5 (1.0 1.0 1.0)))))

(event `self.FireEvent`
  (bind _projectiles (`self.Projectiles`))
  (bind _arrow4 (`self.Arrow4`))
  (bind _arrow5 (`self.Arrow5`))
  (bind _arrow3 (`self.Arrow3`))
  (bind _arrow1 (`self.Arrow1`))
  (bind _arrow2 (`self.Arrow2`))
  (bind _weapionarrow (`self.WeapionArrow`))
  ;[1 1 1] Comment
  (`self.FireProj` (`.ProjectileSize_16_13C10ECE4615C0363B8BE8907C91790E` (break `/Game/StudentWork/enemy/S_TurretBaseStates` (stale `self.ReceiveBeginPlay` _output_get))) _projectiles (`.TurretDamge_10_2C9AE03F4D8927A919688B98DC44852D` (break `/Game/StudentWork/enemy/S_TurretBaseStates` (stale `self.ReceiveBeginPlay` _output_get))) (`SceneComponent.K2_GetComponentLocation` _arrow4) (`SceneComponent.K2_GetComponentRotation` _arrow4))
  (`self.FireProj` (`.ProjectileSize_16_13C10ECE4615C0363B8BE8907C91790E` (break `/Game/StudentWork/enemy/S_TurretBaseStates` (stale `self.ReceiveBeginPlay` _output_get))) _projectiles (`.TurretDamge_10_2C9AE03F4D8927A919688B98DC44852D` (break `/Game/StudentWork/enemy/S_TurretBaseStates` (stale `self.ReceiveBeginPlay` _output_get))) (`SceneComponent.K2_GetComponentLocation` _arrow5) (`SceneComponent.K2_GetComponentRotation` _arrow5))
  (`self.FireProj` (`.ProjectileSize_16_13C10ECE4615C0363B8BE8907C91790E` (break `/Game/StudentWork/enemy/S_TurretBaseStates` (stale `self.ReceiveBeginPlay` _output_get))) _projectiles (`.TurretDamge_10_2C9AE03F4D8927A919688B98DC44852D` (break `/Game/StudentWork/enemy/S_TurretBaseStates` (stale `self.ReceiveBeginPlay` _output_get))) (`SceneComponent.K2_GetComponentLocation` _arrow3) (`SceneComponent.K2_GetComponentRotation` _arrow3))
  (`self.FireProj` (`.ProjectileSize_16_13C10ECE4615C0363B8BE8907C91790E` (break `/Game/StudentWork/enemy/S_TurretBaseStates` (stale `self.ReceiveBeginPlay` _output_get))) _projectiles (`.TurretDamge_10_2C9AE03F4D8927A919688B98DC44852D` (break `/Game/StudentWork/enemy/S_TurretBaseStates` (stale `self.ReceiveBeginPlay` _output_get))) (`SceneComponent.K2_GetComponentLocation` _arrow1) (`SceneComponent.K2_GetComponentRotation` _arrow1))
  (`self.FireProj` (`.ProjectileSize_16_13C10ECE4615C0363B8BE8907C91790E` (break `/Game/StudentWork/enemy/S_TurretBaseStates` (stale `self.ReceiveBeginPlay` _output_get))) _projectiles (`.TurretDamge_10_2C9AE03F4D8927A919688B98DC44852D` (break `/Game/StudentWork/enemy/S_TurretBaseStates` (stale `self.ReceiveBeginPlay` _output_get))) (`SceneComponent.K2_GetComponentLocation` _arrow2) (`SceneComponent.K2_GetComponentRotation` _arrow2))
  (`self.FireProj` (`.ProjectileSize_16_13C10ECE4615C0363B8BE8907C91790E` (break `/Game/StudentWork/enemy/S_TurretBaseStates` (stale `self.ReceiveBeginPlay` _output_get))) _projectiles (`.TurretDamge_10_2C9AE03F4D8927A919688B98DC44852D` (break `/Game/StudentWork/enemy/S_TurretBaseStates` (stale `self.ReceiveBeginPlay` _output_get))) (`SceneComponent.K2_GetComponentLocation` _weapionarrow) (`SceneComponent.K2_GetComponentRotation` _weapionarrow)))

(fn `UserConstructionScript`
  (`parent.UserConstructionScript`))