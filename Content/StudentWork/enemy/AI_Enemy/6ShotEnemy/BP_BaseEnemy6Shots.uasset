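; Six-shot enemy Blueprint that fires a volley of six projectiles at once.
; BeginPlay runs the parent logic, then overrides BaseStates with this variant's stats.
; FireEvent calls FireProj once per weapon arrow component, spawning at that arrow's world transform with the shared projectile and size.
; The AttackDmg input is fed from BaseStates.AttackSpeed rather than a damage field.
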(event `self.ReceiveBeginPlay`
  (`parent.ReceiveBeginPlay`)
  (bind _output_get (set `self.BaseStates` (make `/Game/StudentWork/enemy/S_TurretBaseStates` 250.0 250.0 1500.0 2.5 0.25 (1.0 1.0 1.0)))))

(event `self.FireEvent`
  (bind _projectiles (`self.Projectiles`))
  (bind _weapionarrow1 (`self.WeapionArrow1`))
  (bind _weapionarrow2 (`self.WeapionArrow2`))
  (bind _weapionarrow3 (`self.WeapionArrow3`))
  (bind _weapionarrow4 (`self.WeapionArrow4`))
  (bind _weapionarrow5 (`self.WeapionArrow5`))
  (bind _weapionarrow (`self.WeapionArrow`))
  ;[1 1 1] Comment
  (`self.FireProj` (`.ProjectileSize_16_13C10ECE4615C0363B8BE8907C91790E` (break `/Game/StudentWork/enemy/S_TurretBaseStates` (stale `self.ReceiveBeginPlay` _output_get))) _projectiles (`.AttackSpeed_12_8B4961294720CC25E68449B3DA607308` (break `/Game/StudentWork/enemy/S_TurretBaseStates` (stale `self.ReceiveBeginPlay` _output_get))) (`SceneComponent.K2_GetComponentLocation` _weapionarrow1) (`SceneComponent.K2_GetComponentRotation` _weapionarrow1))
  (`self.FireProj` (`.ProjectileSize_16_13C10ECE4615C0363B8BE8907C91790E` (break `/Game/StudentWork/enemy/S_TurretBaseStates` (stale `self.ReceiveBeginPlay` _output_get))) _projectiles (`.AttackSpeed_12_8B4961294720CC25E68449B3DA607308` (break `/Game/StudentWork/enemy/S_TurretBaseStates` (stale `self.ReceiveBeginPlay` _output_get))) (`SceneComponent.K2_GetComponentLocation` _weapionarrow2) (`SceneComponent.K2_GetComponentRotation` _weapionarrow2))
  (`self.FireProj` (`.ProjectileSize_16_13C10ECE4615C0363B8BE8907C91790E` (break `/Game/StudentWork/enemy/S_TurretBaseStates` (stale `self.ReceiveBeginPlay` _output_get))) _projectiles (`.AttackSpeed_12_8B4961294720CC25E68449B3DA607308` (break `/Game/StudentWork/enemy/S_TurretBaseStates` (stale `self.ReceiveBeginPlay` _output_get))) (`SceneComponent.K2_GetComponentLocation` _weapionarrow3) (`SceneComponent.K2_GetComponentRotation` _weapionarrow3))
  (`self.FireProj` (`.ProjectileSize_16_13C10ECE4615C0363B8BE8907C91790E` (break `/Game/StudentWork/enemy/S_TurretBaseStates` (stale `self.ReceiveBeginPlay` _output_get))) _projectiles (`.AttackSpeed_12_8B4961294720CC25E68449B3DA607308` (break `/Game/StudentWork/enemy/S_TurretBaseStates` (stale `self.ReceiveBeginPlay` _output_get))) (`SceneComponent.K2_GetComponentLocation` _weapionarrow4) (`SceneComponent.K2_GetComponentRotation` _weapionarrow4))
  (`self.FireProj` (`.ProjectileSize_16_13C10ECE4615C0363B8BE8907C91790E` (break `/Game/StudentWork/enemy/S_TurretBaseStates` (stale `self.ReceiveBeginPlay` _output_get))) _projectiles (`.AttackSpeed_12_8B4961294720CC25E68449B3DA607308` (break `/Game/StudentWork/enemy/S_TurretBaseStates` (stale `self.ReceiveBeginPlay` _output_get))) (`SceneComponent.K2_GetComponentLocation` _weapionarrow5) (`SceneComponent.K2_GetComponentRotation` _weapionarrow5))
  (`self.FireProj` (`.ProjectileSize_16_13C10ECE4615C0363B8BE8907C91790E` (break `/Game/StudentWork/enemy/S_TurretBaseStates` (stale `self.ReceiveBeginPlay` _output_get))) _projectiles (`.AttackSpeed_12_8B4961294720CC25E68449B3DA607308` (break `/Game/StudentWork/enemy/S_TurretBaseStates` (stale `self.ReceiveBeginPlay` _output_get))) (`SceneComponent.K2_GetComponentLocation` _weapionarrow) (`SceneComponent.K2_GetComponentRotation` _weapionarrow)))

(fn `UserConstructionScript`
  (`parent.UserConstructionScript`))