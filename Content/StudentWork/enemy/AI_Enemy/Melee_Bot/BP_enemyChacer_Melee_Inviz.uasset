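; Invisible variant of a melee chaser enemy that starts hidden and is revealed on proximity.
; BeginPlay runs the parent logic, then hides the body mesh, weapon, health bar, energy bar and Melee component.
; Any Sphere begin-overlap shows them again, with no filter on the overlapping actor.
; Only visibility is toggled, without propagation to children, and nothing here hides the enemy again after reveal.
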(event `self.ReceiveBeginPlay`
  (`parent.ReceiveBeginPlay`)
  (`self.Set Inviz_1`))

(event `set viz_1`
  (`SceneComponent.SetVisibility` (`self.StaticMesh`) true false)
  (`SceneComponent.SetVisibility` (`self.SM_enemyWeapion`) true false)
  (`SceneComponent.SetVisibility` (`self.HealthBar`) true false)
  (`SceneComponent.SetVisibility` (`self.EnergyBar`) true false)
  (`SceneComponent.SetVisibility` (`self.melee`) true false))

(event `self.Sphere.OnComponentBeginOverlap`
  (params (OverlappedComponent :type "PrimitiveComponent Object Reference") (OtherActor :type "Actor Object Reference") (OtherComp :type "PrimitiveComponent Object Reference") (OtherBodyIndex :type Integer) (bFromSweep :type Boolean) (SweepResult :type "HitResult Structure (by ref)"))
  (`self.set viz_1`))

(event `Set Inviz_1`
  (`SceneComponent.SetVisibility` (`self.StaticMesh`) false false)
  (`SceneComponent.SetVisibility` (`self.SM_enemyWeapion`) false false)
  (`SceneComponent.SetVisibility` (`self.HealthBar`) false false)
  (`SceneComponent.SetVisibility` (`self.EnergyBar`) false false)
  (`SceneComponent.SetVisibility` (`self.melee`) false false))

(fn `UserConstructionScript`
  (`parent.UserConstructionScript`))