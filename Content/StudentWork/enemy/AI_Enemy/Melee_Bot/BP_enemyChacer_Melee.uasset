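; Melee chaser enemy bot that overrides base stats on BeginPlay and builds on inherited movement and fire timers.
; Sphere overlap with the player character sets the target and starts the movement timer.
; Any Box overlap sets a melee-range flag and starts the fire timer; leaving clears the flag.
; While in range, Fire damages the actor stored by the Sphere events and calls an empty animation event.
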(event `self.ReceiveBeginPlay`
  (`parent.ReceiveBeginPlay`)
  (bind _output_get (set `self.BaseStates` (make `/Game/StudentWork/enemy/S_TurretBaseStates` 350.0 350.0 0.0 25.0 0.5))))

(event `self.Sphere.OnComponentBeginOverlap`
  (params (OverlappedComponent :type "PrimitiveComponent Object Reference") (OtherActor :type "Actor Object Reference") (OtherComp :type "PrimitiveComponent Object Reference") (OtherBodyIndex :type Integer) (bFromSweep :type Boolean) (SweepResult :type "HitResult Structure (by ref)"))
  (bind _asbp_player_character (cast `/Game/Blueprints/BP_PlayerCharacter` OtherActor))
  (set `self.Target` _asbp_player_character)
  (`self.StartMovementTimer`)
  (set `self.OtherActor` OtherActor))

(event `self.Sphere.OnComponentEndOverlap`
  (params (OverlappedComponent :type "PrimitiveComponent Object Reference") (OtherActor :type "Actor Object Reference") (OtherComp :type "PrimitiveComponent Object Reference") (OtherBodyIndex :type Integer))
  (set `self.OtherActor` OtherActor))

(event `self.Fire`
  (if (`self.InMeleeRange`)
    (`GameplayStatics.ApplyDamage` (stale `self.Box.OnComponentBeginOverlap` OtherActor) (`.TurretDamge_10_2C9AE03F4D8927A919688B98DC44852D` (break `/Game/StudentWork/enemy/S_TurretBaseStates` (stale `self.ReceiveBeginPlay` _output_get))) null self)
    (`self.Animtion`)))

(event `self.Box.OnComponentBeginOverlap`
  (params (OverlappedComponent :type "PrimitiveComponent Object Reference") (OtherActor :type "Actor Object Reference") (OtherComp :type "PrimitiveComponent Object Reference") (OtherBodyIndex :type Integer) (bFromSweep :type Boolean) (SweepResult :type "HitResult Structure (by ref)"))
  (set `self.InMeleeRange` true)
  (`self.StartFireTimer`))

(event `self.Box.OnComponentEndOverlap`
  (params (OverlappedComponent :type "PrimitiveComponent Object Reference") (OtherActor :type "Actor Object Reference") (OtherComp :type "PrimitiveComponent Object Reference") (OtherBodyIndex :type Integer))
  (set `self.InMeleeRange` false))

(event `Animtion`)

(fn `UserConstructionScript`
  (`parent.UserConstructionScript`))