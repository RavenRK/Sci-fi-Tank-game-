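; BP_EnemyMini_follower is a mini enemy that follows another actor, stored in EmenyToFollow.
; On BeginPlay it sets Movespeed, runs the parent's BeginPlay, fills BaseStates and starts a movement timer.
; Its Move event issues AI MoveTo toward that actor with a small acceptance radius when the reference is valid.
; Nothing in this graph assigns the follow target, and Tick is disabled.
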(event `self.ReceiveBeginPlay`
  (set `self.movespeed?` 0.1)
  (`parent.ReceiveBeginPlay`)
  (set `self.BaseStates` (make `/Game/StudentWork/enemy/S_TurretBaseStates` 150.0 150.0 555.0 15.0 0.3 (1.0 1.0 1.0)))
  (`self.StartMovementTimer`))

(event `self.Move`
  (bind _emenytofollow (`self.EmenyToFollow`))
  ;[1 1 1] new move
  (`/Engine/EditorBlueprintResources/StandardMacros.IsValid` _emenytofollow
    (:`Is Valid`
      (`|AIMoveTo` self (0.0 0.0 0.0) _emenytofollow 25.0))))

(fn `UserConstructionScript`
  (`parent.UserConstructionScript`))