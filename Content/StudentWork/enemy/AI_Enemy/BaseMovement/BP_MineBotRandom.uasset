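; BP_MineBotRandom is a mine bot enemy that wanders randomly and detonates when its target gets close.
; BeginPlay starts a movement timer, and the Move event sends the bot to a random reachable navigation point near its current location via AIMoveTo.
; When Target overlaps the BoomRange component, the bot starts moving toward it and immediately calls Detanate, which is defined outside this graph.
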(event `self.Move`
  (`self.RandomMove`))

(event `self.BoomRange.OnComponentBeginOverlap`
  (params (OverlappedComponent :type "PrimitiveComponent Object Reference") (OtherActor :type "Actor Object Reference") (OtherComp :type "PrimitiveComponent Object Reference") (OtherBodyIndex :type Integer) (bFromSweep :type Boolean) (SweepResult :type "HitResult Structure (by ref)"))
  ;[1 1 1] Comment
  (if (== (`self.Target`) OtherActor)
    (`self.GoAfterPlayer`)
    (`self.detanate`)))

(event `self.ReceiveBeginPlay`
  ;[1 1 1] Comment
  (`parent.ReceiveBeginPlay`)
  (`self.StartMovementTimer`))

(event `GoAfterPlayer`
  (bind _target (`self.Target`))
  ;[1 1 1] chase Player
  (`/Engine/EditorBlueprintResources/StandardMacros.IsValid` _target
    (:`Is Valid`
      (`|AIMoveTo` self (0.0 0.0 0.0) _target 1.0))))

(event `RandomMove`
  ;[1 1 1] Comment
  (`|AIMoveTo` self (`NavigationSystemV1.K2_GetRandomReachablePointInRadius` (`self.K2_GetActorLocation`) 600.0 null null) null 250.0))

(fn `UserConstructionScript`
  (`parent.UserConstructionScript`))