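; Patrolling enemy Blueprint that alternates between walking a looping list of Locations and chasing a Target.
; SetStats fills BaseStates and turn speed, then starts the movement timer.
; Move picks chase or patrol from SeePlayer, both using AIMoveTo, and a successful patrol move advances the index.
; Sphere overlaps with any actor toggle SeePlayer: begin clears it and end sets it, so chasing follows an exit from the sphere.
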(event `self.Set Stats`
  (set `self.BaseStates` (make `/Game/StudentWork/enemy/S_TurretBaseStates` 450.0 450.0 2000.0 5.0 0.2 (1.5 1.5 1.5)))
  (set `self.Tern_Speed` 3.5)
  (`self.StartMovementTimer`))

(event `self.Sphere.OnComponentBeginOverlap`
  (params (OverlappedComponent :type "PrimitiveComponent Object Reference") (OtherActor :type "Actor Object Reference") (OtherComp :type "PrimitiveComponent Object Reference") (OtherBodyIndex :type Integer) (bFromSweep :type Boolean) (SweepResult :type "HitResult Structure (by ref)"))
  (set `self.SeePlayer` false))

(event `self.Sphere.OnComponentEndOverlap`
  (params (OverlappedComponent :type "PrimitiveComponent Object Reference") (OtherActor :type "Actor Object Reference") (OtherComp :type "PrimitiveComponent Object Reference") (OtherBodyIndex :type Integer))
  (set `self.SeePlayer` true))

(event `self.ReceiveTick`
  (params (DeltaSeconds :type "Float (single-precision)"))
  (`parent.ReceiveTick` DeltaSeconds))

(event `ChasePlayer`
  (bind _target (`self.Target`))
  ;[1 1 1] see player
  (`/Engine/EditorBlueprintResources/StandardMacros.IsValid` _target
    (:`Is Valid`
      (`|AIMoveTo` self (0.0 0.0 0.0) _target))))

(event `self.Move`
  ;[1 1 1] control
  (if (`self.SeePlayer`)
    (`self.ChasePlayer`)
    (else
      (`self.PatrolPionts`))))

(event `PatrolPionts`
  (bind _locations (`self.Locations`))
  (bind _locationscount (`self.LocationsCount`))
  ;[1 1 1] patrol
  (`|AIMoveTo` self (0.0 0.0 0.0) (`|GetArrayItem` _locations (`self.LocationsCount`)) 100.0
    (:`OnSuccess`
      (`/Engine/EditorBlueprintResources/StandardMacros.IncrementInt` _locationscount
        (:`  `
          (if (== (`KismetArrayLibrary.Array_Length` _locations) _locationscount)
            (set `self.LocationsCount` 0)))))))

(fn `UserConstructionScript`
  (`parent.UserConstructionScript`))