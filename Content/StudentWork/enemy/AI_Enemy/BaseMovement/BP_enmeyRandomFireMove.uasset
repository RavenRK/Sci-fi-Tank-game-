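; Enemy Blueprint variant whose weapon turns independently of the player, built on parent enemy logic for BeginPlay, Tick and construction.
; SetStats fills the base stats and power cost, sizes the sphere to the attack range and enables attacking.
; TurretFollowPlayer smoothly interpolates weapon yaw toward a look-at of a random unit vector, used as a world position and therefore near the world origin.
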(event `self.ReceiveBeginPlay`
  ;[1 1 1] other
  (`parent.ReceiveBeginPlay`))

(event `self.Set Stats`
  ;[1 1 1] other
  (bind _output_get (set `self.BaseStates` (make `/Game/StudentWork/enemy/S_TurretBaseStates` 500.0 500.0 3000.0 2.5 0.4 (1.0 1.0 1.0))))
  (set `self.Power_Cost` 1.0)
  (`SphereComponent.SetSphereRadius` (`self.Sphere`) (`.AttackRange_17_03E391084C5EA2C1EDA27592414CA756` (break `/Game/StudentWork/enemy/S_TurretBaseStates` _output_get)) true)
  (set `self.CanAttack` true))

(event `self.ReceiveTick`
  (params (DeltaSeconds :type "Float (single-precision)"))
  ;[1 1 1] other
  (`parent.ReceiveTick` DeltaSeconds))

(event `self.TurretFollow_player`
  (bind _sm_enemyweapion (`self.SM_enemyWeapion`))
  (bind (_returnvalue_roll _returnvalue_pitch _returnvalue_yaw) (`KismetMathLibrary.BreakRotator` (`KismetMathLibrary.FindLookAtRotation` (`SceneComponent.K2_GetComponentLocation` _sm_enemyweapion) (`KismetMathLibrary.Conv_RotatorToVector` (`KismetMathLibrary.RandomRotator` false)))))
  ;[1 1 1] new follow player
  (`SceneComponent.K2_SetWorldRotation` _sm_enemyweapion (`KismetMathLibrary.RInterpTo` (`SceneComponent.K2_GetComponentRotation` _sm_enemyweapion) (`KismetMathLibrary.MakeRotator` 0.0 0.0 _returnvalue_yaw) (`GameplayStatics.GetWorldDeltaSeconds`) 1.0) false false))

(fn `UserConstructionScript`
  (`parent.UserConstructionScript`))