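; BP_MineBot is an enemy mine bot that self-destructs when its target gets close.
; On BeginPlay it calls its parent and sets its base stats.
; When the inherited-style Target overlaps BoomRange, a timeline drives the flashTimer parameter on a dynamic flashing material created in the construction script.
; When the timeline finishes, it applies radial damage at the mesh location, prints a debug message and destroys itself.
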(event `self.ReceiveBeginPlay`
  (`parent.ReceiveBeginPlay`)
  (set `self.BaseStates` (make `/Game/StudentWork/enemy/S_TurretBaseStates` 500.0 500.0 1000.0)))

(event `self.BoomRange.OnComponentBeginOverlap`
  (params (OverlappedComponent :type "PrimitiveComponent Object Reference") (OtherActor :type "Actor Object Reference") (OtherComp :type "PrimitiveComponent Object Reference") (OtherBodyIndex :type Integer) (bFromSweep :type Boolean) (SweepResult :type "HitResult Structure (by ref)"))
  (if (== (`self.Target`) OtherActor)
    (`self.detanate`)))

(event `detanate`
  ;[1 1 1] Detanate
  (bind (_direction _newtrack_0) (`Timeline|Timeline`)
    (:`Update`
      (`MaterialInstanceDynamic.SetScalarParameterValue` (`self.FlashMat`) "flashTimer" _newtrack_0))
    (:`Finished`
      (`GameplayStatics.ApplyRadialDamage` :`BaseDamage` 50.0 :`Origin` (`SceneComponent.K2_GetComponentLocation` (`self.StaticMesh`)) :`DamageRadius` 500.0 :`DamageCauser` self :`InstigatedByController` null)
      (`KismetSystemLibrary.PrintString` "BOOOOOOM")
      (`self.K2_DestroyActor`))))

(fn `UserConstructionScript`
  (bind _returnvalue (`PrimitiveComponent.CreateDynamicMaterialInstance` (`self.SM_enemyWeapion`) 1 "/Game/StudentWork/enemy/AI_Enemy/M_FlashingMat.M_FlashingMat" "None"))
  (set `self.FlashMat` _returnvalue))