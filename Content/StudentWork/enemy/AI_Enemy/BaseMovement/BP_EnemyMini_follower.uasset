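; BP_EnemyMini_follower is a mini enemy variant that follows another enemy.
; It overrides SetStats to assign its move speed and base states, then starts the movement timer.
; Its Move event uses AI Move To to head toward the referenced EmenyToFollow actor, stopping within an acceptance radius, and does nothing when that reference is invalid.
; BeginPlay and construction defer to the parent, and Tick is disabled.
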(event `self.Set Stats`
  (set `self.movespeed?` 0.1)
  (set `self.BaseStates` (make `/Game/StudentWork/enemy/S_TurretBaseStates` 200.0 200.0 1500.0 2.5 0.5 (1.0 1.0 1.0)))
  (`self.StartMovementTimer`))

(event `self.ReceiveBeginPlay`
  (`parent.ReceiveBeginPlay`))

(event `self.Move`
  (bind _emenytofollow (`self.EmenyToFollow`))
  ;[1 1 1] new move
  (`/Engine/EditorBlueprintResources/StandardMacros.IsValid` _emenytofollow
    (:`Is Valid`
      (`|AIMoveTo` self (0.0 0.0 0.0) _emenytofollow 100.0))))

(fn `UserConstructionScript`
  (`parent.UserConstructionScript`))