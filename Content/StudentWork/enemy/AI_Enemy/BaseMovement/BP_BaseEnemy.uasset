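; BP_BaseEnemy is a base turreted enemy that fires projectiles at the player, takes damage and explodes on death.
; A player entering the range sphere starts looping move and fire timers, though Move only prints a debug message.
; Tick turns the weapon toward the overlapping actor and the hull along velocity.
; Firing drains power, pausing to recharge when empty, and a stats struct drives combat values and the widget's health bar.
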(event `exblode`
  ;[1 1 1] Dead VFX
  (`NiagaraFunctionLibrary.SpawnSystemAtLocation` "/Game/StudentWork/enemy/NS_Explode_blue.NS_Explode_blue" (`SceneComponent.K2_GetComponentLocation` (`self.CapsuleComponent`))))

(event `TurretFollow_player`
  (bind _sm_enemyweapion (`self.SM_enemyWeapion`))
  (bind _otheractor (`self.OtherActor`))
  (bind (_returnvalue_roll _returnvalue_pitch _returnvalue_yaw) (`KismetMathLibrary.BreakRotator` (`KismetMathLibrary.FindLookAtRotation` (`SceneComponent.K2_GetComponentLocation` _sm_enemyweapion) (`self.K2_GetActorLocation` _otheractor))))
  ;[0.1323 0.02002 0.1771] TurretFunctions
  ;;[1 1 1] follow
  (`/Engine/EditorBlueprintResources/StandardMacros.IsValid` _otheractor
    (:`Is Valid`
      (`SceneComponent.K2_SetWorldRotation` _sm_enemyweapion (`KismetMathLibrary.RInterpTo` (`SceneComponent.K2_GetComponentRotation` _sm_enemyweapion) (`KismetMathLibrary.MakeRotator` _returnvalue_roll _returnvalue_pitch _returnvalue_yaw) (`GameplayStatics.GetWorldDeltaSeconds`) (`self.Tern_Speed`)) false false))))

(event `self.Sphere.OnComponentBeginOverlap`
  (params (OverlappedComponent :type "PrimitiveComponent Object Reference") (OtherActor :type "Actor Object Reference") (OtherComp :type "PrimitiveComponent Object Reference") (OtherBodyIndex :type Integer) (bFromSweep :type Boolean) (SweepResult :type "HitResult Structure (by ref)"))
  ;[0.1619 1 0.1942] Base AI
  ;;[0.3353 1 0.3596] what to do when overlap
  (bind _asbp_player_character (cast `/Game/Blueprints/BP_PlayerCharacter` OtherActor))
  (set `self.Target` _asbp_player_character)
  (`self.StartMovementTimer`)
  ;[0.1323 0.02002 0.1771] TurretFunctions
  ;;[1 0.01036 0.02031] can attack
  (set `self.OtherActor` OtherActor)
  (set `self.CanAttack` true)
  (`KismetSystemLibrary.PrintString` "can fire")
  (`self.StartFireTimer`))

(event `self.Sphere.OnComponentEndOverlap`
  (params (OverlappedComponent :type "PrimitiveComponent Object Reference") (OtherActor :type "Actor Object Reference") (OtherComp :type "PrimitiveComponent Object Reference") (OtherBodyIndex :type Integer))
  ;[0.1323 0.02002 0.1771] TurretFunctions
  ;;[1 0.01036 0.02031] can attack
  (set `self.OtherActor` OtherActor)
  (set `self.CanAttack` false)
  (`KismetSystemLibrary.PrintString` "cant fire"))

(event `StartMovementTimer`
  ;[0.1619 1 0.1942] Base AI
  ;;[0.3666 1 0.4332] set moveing timer
  (bind _returnvalue (`KismetSystemLibrary.K2_SetTimerDelegate` (delegate `Move`) (`self.movespeed?`) true))
  (set `self.MovementTimerr` _returnvalue))

(event `Move`
  ;[0.1619 1 0.1942] Base AI
  ;;[0.3666 1 0.4332] set moveing timer
  (`KismetSystemLibrary.PrintString` "moveing"))

(event `Set Stats`
  ;[1 1 1] Stats
  (set `self.BaseStates` (make `/Game/StudentWork/enemy/S_TurretBaseStates` 250.0 250.0 1000.0 2.5 0.5 (1.0 1.0 1.0))))

(event `StartFireTimer`
  (bind (_basestates_currenthealth _basestates_maxhealth _basestates_attackrange _basestates_turretdamge _basestates_attackspeed _basestates_projectilesize) (break `/Game/StudentWork/enemy/S_TurretBaseStates` (`self.BaseStates`)))
  ;[0.1323 0.02002 0.1771] TurretFunctions
  ;;[1 0.1036 0.09369] attack timer
  (bind _returnvalue (`KismetSystemLibrary.K2_SetTimerDelegate` (delegate `Fire`) _basestates_attackspeed true))
  (set `self.AttackTimer` _returnvalue))

(event `self.ReceiveTick`
  (params (DeltaSeconds :type "Float (single-precision)"))
  ;[0.1323 0.02002 0.1771] TurretFunctions
  ;;[1 0.6029 0] event tick
  (`self.TurretFollow_player`)
  (`self.HullToFace`))

(event `Fire`
  ;[0.1323 0.02002 0.1771] TurretFunctions
  ;;[1 0.1036 0.09369] attack timer
  (if (`self.CanAttack`)
    (`self.PowerUpdate`)
    (`self.PowerCheck`)
    (`self.FireEvent`)))

(event `Event Setup UI`
  ;[1 1 1] UI
  ;;[0.1146 0.8702 1] UI set Up
  (message `/Game/StudentWork/enemy/UI/BP_setUIOwner.setUIOwner` (`WidgetComponent.GetUserWidgetObject` (`self.HealthBar`)) self)
  (`self.Health Update`)
  (`self.PowerUpdate`))

(event `self.ReceiveAnyDamage`
  (params (Damage :type "Float (single-precision)") (DamageType :type "DamageType Object Reference") (InstigatedBy :type "Controller Object Reference") (DamageCauser :type "Actor Object Reference"))
  (bind (_basestates_currenthealth _basestates_maxhealth _basestates_attackrange _basestates_turretdamge _basestates_attackspeed _basestates_projectilesize) (break `/Game/StudentWork/enemy/S_TurretBaseStates` (`self.BaseStates`)))
  ;[0.1323 0.02002 0.1771] TurretFunctions
  ;;[0.9843 0.492 1] Take DMG
  (if (not (`self.Dead`))
    (bind _structout (setmembers `/Game/StudentWork/enemy/S_TurretBaseStates` :`StructRef` (`self.BaseStates`) :`CurrentHealth` (`KismetMathLibrary.FClamp` (- _basestates_currenthealth Damage) 0.0 _basestates_maxhealth)))
    (`KismetSystemLibrary.PrintString` (`KismetStringLibrary.Conv_DoubleToString` (break `/Game/StudentWork/enemy/S_TurretBaseStates` _structout)))
    (`self.Health Update`)
    (if (<= _basestates_currenthealth 0.0)
      (set `self.CanAttack` false)
      (set `self.Dead` true)
      (`self.exblode`)
      (`self.K2_DestroyActor`))))

(event `Health Update`
  ;[1 1 1] UI
  ;;[0.12 0.7579 1] HealthUpdate
  (`self.HealthPercentage` (`self.Get Health Percentage`)))

(event `PowerUpdate`
  ;[1 1 1] UI
  ;;[0.1758 0.7153 1] powerUpdate
  (`self.PowerPercentage` (`self.Power_ammo`)))

(event `self.ReceiveBeginPlay`
  (bind (_basestates_currenthealth _basestates_maxhealth _basestates_attackrange _basestates_turretdamge _basestates_attackspeed _basestates_projectilesize) (break `/Game/StudentWork/enemy/S_TurretBaseStates` (`self.BaseStates`)))
  ;[0.1323 0.02002 0.1771] TurretFunctions
  ;;[0.9843 0.492 1] Take DMG
  ;;;[0.9676 0.04473 1] Begin
  (`self.Event Setup UI`)
  (`self.Set Stats`)
  (`SphereComponent.SetSphereRadius` (`self.Sphere`) _basestates_attackrange true))

(event `FireEvent`
  (bind _weapionarrow (`self.WeapionArrow`))
  (bind (_basestates_currenthealth _basestates_maxhealth _basestates_attackrange _basestates_turretdamge _basestates_attackspeed _basestates_projectilesize) (break `/Game/StudentWork/enemy/S_TurretBaseStates` (`self.BaseStates`)))
  ;[0.1323 0.02002 0.1771] TurretFunctions
  ;;[0.9843 0.492 1] Take DMG
  (`self.FireProj` _basestates_projectilesize (`self.Projectiles`) _basestates_turretdamge (`SceneComponent.K2_GetComponentLocation` _weapionarrow) (`SceneComponent.K2_GetComponentRotation` _weapionarrow)))

(event `PowerCheck`
  ;[1 0.01036 0.02031] Power/ammo check
  (if (<= (`self.Power_ammo`) 0.0)
    (set `self.CanAttack` false)
    (`KismetSystemLibrary.Delay` 2.0)
    (set `self.Power_ammo` 100.0)
    (set `self.CanAttack` true)
    (else
      (set `self.Power_ammo` (- (`self.Power_ammo`) (`self.Power_Cost`))))))

(event `HullToFace`
  (bind _returnvalue (`self.GetVelocity`))
  (bind _staticmesh (`self.StaticMesh`))
  (bind (_returnvalue_roll _returnvalue_pitch _returnvalue_yaw) (`KismetMathLibrary.BreakRotator` (`KismetMathLibrary.MakeRotFromX` _returnvalue)))
  ;[1 1 1] Hull to face
  (if (> (`KismetMathLibrary.VSize` _returnvalue) 0.0)
    (`SceneComponent.K2_SetWorldRotation` _staticmesh (`KismetMathLibrary.RInterpTo` (`SceneComponent.K2_GetComponentRotation` _staticmesh) (`KismetMathLibrary.MakeRotator` 0.0 0.0 _returnvalue_yaw) (`GameplayStatics.GetWorldDeltaSeconds`) 2.0) false false)))

(fn `FireProj`
  (params (ProJScale :type "Vector Structure" :default (1.0 1.0 0.0)) (ProJ :type "Actor Class Reference (by ref)") (AttackDmg :type "Float (double-precision)") (SpawnLocation :type "Vector Structure") (SpawnRotation :type "Rotator Structure"))
  (bind _asbp_base_projectile (castclass `/Game/StudentWork/enemy/turret/BP_BaseProjectile` ProJ))
  (`|SpawnActorFromClass` _asbp_base_projectile (`KismetMathLibrary.MakeTransform` SpawnLocation SpawnRotation ProJScale) "Undefined" "MultiplyWithRoot" null AttackDmg null)
  (`NiagaraFunctionLibrary.SpawnSystemAtLocation` "/Game/StudentWork/enemy/turret/VFX/NS_fireEffect.NS_fireEffect" SpawnLocation SpawnRotation))

(fn `Get Health Percentage`
  (returns (ReturnValue :type "Float (double-precision)"))
  (bind (_basestates_currenthealth _basestates_maxhealth) (break `/Game/StudentWork/enemy/S_TurretBaseStates` (`self.BaseStates`)))
  (return (/ _basestates_currenthealth _basestates_maxhealth)))

(fn `UserConstructionScript`
  (`SceneComponent.K2_SetWorldRotation` (`self.StaticMesh`) (`SceneComponent.K2_GetComponentRotation` (`self.CapsuleComponent`)) false false))