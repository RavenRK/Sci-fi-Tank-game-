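; BP_MachenGunT is a machine gun turret enemy Blueprint that sets its own base stats and spins its gun rod while something overlaps its sphere.
; BeginPlay fills BaseStates before calling the parent, which also receives Tick and construction.
; Sphere begin overlap plays a Timeline that maps its track to rod pitch over 360 degrees.
; Any end overlap stops the Timeline, with no check on the overlapping actor.
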(event `self.ReceiveBeginPlay`
  ;[0.864 0.7081 1] set base stats
  (set `self.BaseStates` (make `/Game/StudentWork/enemy/S_TurretBaseStates` 500.0 500.0 1250.0 2.5 0.07 (0.5 1.0 0.5)))
  (`parent.ReceiveBeginPlay`))

(event `self.ReceiveTick`
  (params (DeltaSeconds :type "Float (single-precision)"))
  ;[0.864 0.7081 1] set base stats
  (`parent.ReceiveTick` DeltaSeconds))

(event `self.Sphere.OnComponentBeginOverlap`
  (params (OverlappedComponent :type "PrimitiveComponent Object Reference") (OtherActor :type "Actor Object Reference") (OtherComp :type "PrimitiveComponent Object Reference") (OtherBodyIndex :type Integer) (bFromSweep :type Boolean) (SweepResult :type "HitResult Structure (by ref)"))
  ;[1 1 1] animtion for sbining
  (bind (_direction _newtrack_0) (`Timeline|Timeline` :!label _label)
    (:`Update`
      (`SceneComponent.K2_SetRelativeRotation` (`self.machenGun_rode`) (`KismetMathLibrary.MakeRotator` 0.0 (* _newtrack_0 360.0)) false false))))

(event `self.Sphere.OnComponentEndOverlap`
  (params (OverlappedComponent :type "PrimitiveComponent Object Reference") (OtherActor :type "Actor Object Reference") (OtherComp :type "PrimitiveComponent Object Reference") (OtherBodyIndex :type Integer))
  ;[1 1 1] animtion for sbining
  (goto _label :!via `Stop`))

(fn `UserConstructionScript`
  (`parent.UserConstructionScript`))