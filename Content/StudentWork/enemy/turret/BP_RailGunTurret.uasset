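; Rail gun turret enemy, a child Blueprint that sets its own base stats and layers charge-up visuals onto the parent turret logic.
; While CanAttack is false, Tick re-arms a looping one-second timer every frame.
; When the timer fires, it spawns two gather-energy Niagara systems at Arrow1, then uses delays to nudge GunPipe along local X and back.
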(event `self.ReceiveBeginPlay`
  (set `self.BaseStates` (make `/Game/StudentWork/enemy/S_TurretBaseStates` 350.0 350.0 1050.0 35.0 1.0 (6.0 3.0 3.0)))
  (`parent.ReceiveBeginPlay`))

(event `self.ReceiveTick`
  (params (DeltaSeconds :type "Float (single-precision)"))
  (`parent.ReceiveTick` DeltaSeconds)
  (if (not (`self.CanAttack`))
    (`self.GatherEvent(VFX)`)))

(event `GatherEvent(VFX)`
  ;[1 1 1] VFX and animtions
  (bind _returnvalue (`KismetSystemLibrary.K2_SetTimerDelegate` (delegate `VFXTimer`) 1.0 true))
  (set `self.FireTimer` _returnvalue))

(event `VFXTimer`
  (bind _arrow1 (`self.Arrow1`))
  (bind _returnvalue (`SceneComponent.K2_GetComponentLocation` _arrow1))
  (bind _returnvalue_2 (`SceneComponent.K2_GetComponentRotation` _arrow1))
  ;[1 1 1] VFX and animtions
  (`NiagaraFunctionLibrary.SpawnSystemAtLocation` "/Game/StudentWork/enemy/turret/VFX/NS_GatherEnengy.NS_GatherEnengy" _returnvalue _returnvalue_2)
  (`NiagaraFunctionLibrary.SpawnSystemAtLocation` "/Game/StudentWork/enemy/turret/VFX/NS_GatherEnengy.NS_GatherEnengy" _returnvalue _returnvalue_2)
  (`KismetSystemLibrary.Delay` 0.9)
  (`SceneComponent.K2_AddLocalOffset` (`self.GunPipe`) (`KismetMathLibrary.MakeVector` (+ 10.0 0.0)) false false)
  (`KismetSystemLibrary.Delay` 0.1)
  (`SceneComponent.K2_AddLocalOffset` (`self.GunPipe`) (`KismetMathLibrary.MakeVector` (+ -10.0 0.0)) false false))

(fn `UserConstructionScript`
  (`parent.UserConstructionScript`))