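; Base projectile actor, filed with the turret enemy, that damages whatever its static mesh hits.
; On component hit it applies its Damage value to the other actor, then calls the AfterApplyDMG event.
; That event spawns the HitEffect system at the projectile's location and destroys the actor only if the CanBeDestory flag is set.
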(event `self.StaticMesh.OnComponentHit`
  (params (HitComponent :type "PrimitiveComponent Object Reference") (OtherActor :type "Actor Object Reference") (OtherComp :type "PrimitiveComponent Object Reference") (NormalImpulse :type "Vector Structure") (Hit :type "HitResult Structure (by ref)"))
  (bind _output_get (set `self.Other Actor` OtherActor))
  (`GameplayStatics.ApplyDamage` _output_get (`self.Damage`))
  (`self.AfterApplyDMG`))

(event `AfterApplyDMG`
  (`NiagaraFunctionLibrary.SpawnSystemAtLocation` (`self.HitEffect`) (`self.K2_GetActorLocation`))
  (if (`self.CanBeDestory`)
    (`self.K2_DestroyActor`)))

(fn `UserConstructionScript`)