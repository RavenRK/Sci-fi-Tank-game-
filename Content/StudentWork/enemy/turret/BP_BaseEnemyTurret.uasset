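; Base enemy turret that shoots at actors entering its range sphere, with stats driven by the BaseStates struct.
; Overlap starts a looping fire timer, while Tick smoothly rotates the turret toward the last overlapping actor.
; Each shot spawns a projectile and muzzle effect and drains Power, with a reload delay once empty.
; Damage lowers clamped health, updates UI through power and health calls, and explodes the turret at zero.
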(event `StartFireTimer`
  (bind (_basestates_currenthealth _basestates_maxhealth _basestates_attackrange _basestates_turretdamge _basestates_attackspeed _basestates_projectilesize) (break `/Game/StudentWork/enemy/S_TurretBaseStates` (`self.BaseStates`)))
  ;[1 1 1] fire Proj
  (bind _returnvalue (`KismetSystemLibrary.K2_SetTimerDelegate` (delegate `fire`) _basestates_attackspeed true))
  (set `self.attackTimer` _returnvalue))

(event `PowerCheck`
  ;[1 1 1] powercheck
  (if (<= (`self.Power`) 0.0)
    (set `self.CanAttack` false)
    (`KismetSystemLibrary.Delay` (`self.Reload_Time`))
    (set `self.Power` 100.0)
    (set `self.CanAttack` true)
    (else
      (set `self.Power` (- (`self.Power`) (`self.powerCost`))))))

(event `fire`
  (bind (_basestates_currenthealth _basestates_maxhealth _basestates_attackrange _basestates_turretdamge _basestates_attackspeed _basestates_projectilesize) (break `/Game/StudentWork/enemy/S_TurretBaseStates` (`self.BaseStates`)))
  ;[1 1 1] fire Proj
  (if (`self.CanAttack`)
    (`self.EnergyUpdate`)
    (`self.PowerCheck`)
    (`self.Fire_Projectile` _basestates_projectilesize (`self.Projectiles`) _basestates_turretdamge)))

(event `self.Sphere.OnComponentBeginOverlap`
  (params (OverlappedComponent :type "PrimitiveComponent Object Reference") (OtherActor :type "Actor Object Reference") (OtherComp :type "PrimitiveComponent Object Reference") (OtherBodyIndex :type Integer) (bFromSweep :type Boolean) (SweepResult :type "HitResult Structure (by ref)"))
  ;[1 1 1] can attack
  (set `self.OtherActor` OtherActor)
  (set `self.CanAttack` true)
  (`self.StartFireTimer`))

(event `self.ReceiveTick`
  (params (DeltaSeconds :type "Float (single-precision)"))
  ;[0.1739 0.4226 1] event tick ( follow )
  (`self.Follow_player`))

(event `Follow_player`
  (bind _otheractor (`self.OtherActor`))
  (bind _turret (`self.turret`))
  (bind (_returnvalue_roll _returnvalue_pitch _returnvalue_yaw) (`KismetMathLibrary.BreakRotator` (`KismetMathLibrary.FindLookAtRotation` (`SceneComponent.K2_GetComponentLocation` (`self.turret`)) (`self.K2_GetActorLocation` _otheractor))))
  ;[0.5021 0.5631 1] EVENT follow player
  (`/Engine/EditorBlueprintResources/StandardMacros.IsValid` _otheractor
    (:`Is Valid`
      (`SceneComponent.K2_SetWorldRotation` _turret (`KismetMathLibrary.RInterpTo` (`SceneComponent.K2_GetComponentRotation` _turret) (`KismetMathLibrary.MakeRotator` _returnvalue_roll _returnvalue_pitch _returnvalue_yaw) (`GameplayStatics.GetWorldDeltaSeconds`) 4.0) false false))))

(event `self.Sphere.OnComponentEndOverlap`
  (params (OverlappedComponent :type "PrimitiveComponent Object Reference") (OtherActor :type "Actor Object Reference") (OtherComp :type "PrimitiveComponent Object Reference") (OtherBodyIndex :type Integer))
  ;[1 1 1] can attack
  (set `self.OtherActor` OtherActor)
  (set `self.CanAttack` false)
  (`KismetSystemLibrary.PrintString` "cant fire"))

(event `self.ReceiveAnyDamage`
  (params (Damage :type "Float (single-precision)") (DamageType :type "DamageType Object Reference") (InstigatedBy :type "Controller Object Reference") (DamageCauser :type "Actor Object Reference"))
  (bind (_basestates_currenthealth _basestates_maxhealth _basestates_attackrange) (break `/Game/StudentWork/enemy/S_TurretBaseStates` (`self.BaseStates`)))
  ;[1 1 1] Take DMG
  (if (not (`self.Dead`))
    (setmembers `/Game/StudentWork/enemy/S_TurretBaseStates` :`StructRef` (`self.BaseStates`) :`CurrentHealth` (`KismetMathLibrary.FClamp` (- _basestates_currenthealth Damage) 0.0 _basestates_maxhealth))
    (`self.HealthUpdate`)
    (if (<= _basestates_currenthealth 0.0)
      (set `self.CanAttack` false)
      (set `self.Dead` true)
      (`NiagaraFunctionLibrary.SpawnSystemAtLocation` "/Game/StudentWork/enemy/NS_Explode_blue.NS_Explode_blue" (`SceneComponent.K2_GetComponentLocation` (`self.Box`)))
      (`self.K2_DestroyActor`))))

(event `self.ReceiveBeginPlay`
  (bind (_basestates_currenthealth _basestates_maxhealth _basestates_attackrange) (break `/Game/StudentWork/enemy/S_TurretBaseStates` (`self.BaseStates`)))
  ;[1 1 1] Take DMG
  ;;[1 0 0.007639] begin play
  (`self.Event Setup UI`)
  (`SphereComponent.SetSphereRadius` (`self.Sphere`) _basestates_attackrange true))

(event `EnergyUpdate`
  ;[0.6243 0.7112 1] UI
  ;;[1 1 1] Power Update
  (`self.PowerPercentage` (`self.Power`)))

(event `HealthUpdate`
  ;[0.6243 0.7112 1] UI
  ;;[1 1 1] Health update
  (`self.HealthPercentage` (`self.GetHealthPercentage`)))

(event `Event Setup UI`
  ;[0.6243 0.7112 1] UI
  ;;[1 1 1] set UI owner
  (message `/Game/StudentWork/enemy/UI/BP_setUIOwner.setUIOwner` (`WidgetComponent.GetUserWidgetObject` (`self.HealthBar`)) self)
  (`self.HealthUpdate`))

(fn `Fire_Projectile`
  (params (ProjectileScale :type "Vector Structure" :default (1.0 1.0 0.0)) (Projectles :type "Actor Class Reference (by ref)") (AttackDmg :type "Float (double-precision)" :default 5.0))
  (bind _arrow (`self.Arrow`))
  (bind _returnvalue (`SceneComponent.K2_GetComponentLocation` _arrow))
  (bind _returnvalue_2 (`SceneComponent.K2_GetComponentRotation` _arrow))
  ;[1 1 1] spawn projectile/vfx and sound
  (bind _asbp_base_projectile (castclass `/Game/StudentWork/enemy/turret/BP_BaseProjectile` Projectles))
  (`|SpawnActorFromClass` _asbp_base_projectile (`KismetMathLibrary.MakeTransform` _returnvalue _returnvalue_2 ProjectileScale) "Undefined" "MultiplyWithRoot" null AttackDmg null)
  (`NiagaraFunctionLibrary.SpawnSystemAtLocation` "/Game/StudentWork/enemy/turret/VFX/NS_fireEffect.NS_fireEffect" _returnvalue _returnvalue_2))

(fn `GetHealthPercentage`
  (returns (ReturnValue :type "Float (double-precision)"))
  (bind (_basestates_currenthealth _basestates_maxhealth) (break `/Game/StudentWork/enemy/S_TurretBaseStates` (`self.BaseStates`)))
  (return (/ _basestates_currenthealth _basestates_maxhealth)))

(fn `UserConstructionScript`)