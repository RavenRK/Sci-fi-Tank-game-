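; BP_AttackSpeed is a pickup actor for what its name indicates is an attack speed power-up.
; When a BP_PlayerCharacter overlaps its Capsule, it calls that character's machine gun, shotgun and railgun power-up functions, then destroys itself.
; A looping timer started on BeginPlay spins the Cube around its yaw axis by a fixed step per call, so the animation does not use Tick.
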(event `self.Capsule.OnComponentBeginOverlap`
  (params (OverlappedComponent :type "PrimitiveComponent Object Reference") (OtherActor :type "Actor Object Reference") (OtherComp :type "PrimitiveComponent Object Reference") (OtherBodyIndex :type Integer) (bFromSweep :type Boolean) (SweepResult :type "HitResult Structure (by ref)"))
  (bind _asbp_player_character (cast `/Game/Blueprints/BP_PlayerCharacter` OtherActor))
  (`/Game/Blueprints/BP_PlayerCharacter.MachenGun_powerUp` _asbp_player_character)
  (`/Game/Blueprints/BP_PlayerCharacter.ShotGunPowerUp` _asbp_player_character)
  (`/Game/Blueprints/BP_PlayerCharacter.RailGunPowerUp` _asbp_player_character)
  (`self.K2_DestroyActor`))

(event `StartAnimtionTimer`
  ;[1 1 1] Animtion
  (bind _returnvalue (`KismetSystemLibrary.K2_SetTimerDelegate` (delegate `StartAnimation`) 0.03 true))
  (set `self.AnimtionTimer` _returnvalue))

(event `self.ReceiveBeginPlay`
  (`self.StartAnimtionTimer`))

(event `StartAnimation`
  ;[1 1 1] Animtion
  (`SceneComponent.K2_AddWorldRotation` (`self.Cube`) (struct :`Yaw` 7.0) false false))

(fn `UserConstructionScript`)