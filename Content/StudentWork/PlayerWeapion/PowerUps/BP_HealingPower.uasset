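; BP_HealingPower is a healing power-up shown as a cube that a looping timer keeps spinning.
; Overlapping its capsule stores the other actor, unfiltered, and starts a looping timer that applies negative damage to it as healing.
; A delay clears the healing timer after ten seconds, and the power-up remains in the world.
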(event `self.ReceiveBeginPlay`
  (`self.StartAnimtionTimer`))

(event `self.Capsule.OnComponentBeginOverlap`
  (params (OverlappedComponent :type "PrimitiveComponent Object Reference") (OtherActor :type "Actor Object Reference") (OtherComp :type "PrimitiveComponent Object Reference") (OtherBodyIndex :type Integer) (bFromSweep :type Boolean) (SweepResult :type "HitResult Structure (by ref)"))
  (set `self.Other Actor` OtherActor)
  (`self.StarthealingTimer`)
  (`KismetSystemLibrary.Delay` 10.0)
  (`KismetSystemLibrary.K2_ClearAndInvalidateTimerHandle` (`self.healingTimer`)))

(event `StartHealingTimer`
  ;[1 1 1] Healing tick
  (bind _returnvalue (`KismetSystemLibrary.K2_SetTimerDelegate` (delegate `HealingTick`) 0.5 true))
  (set `self.healingTimer` _returnvalue))

(event `StartAnimtionTimer`
  ;[1 1 1] Animtion
  (bind _returnvalue (`KismetSystemLibrary.K2_SetTimerDelegate` (delegate `StartAnimation`) 0.03 true))
  (set `self.AnimtionTimer` _returnvalue))

(event `HealingTick`
  ;[1 1 1] Healing tick
  (`GameplayStatics.ApplyDamage` (`self.Other Actor`) -2.0))

(event `StartAnimation`
  ;[1 1 1] Animtion
  (`SceneComponent.K2_AddWorldRotation` (`self.Cube`) (struct :`Yaw` 7.0) false false))

(fn `UserConstructionScript`)