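; Player weapon projectile that damages whatever its static mesh hits and expires after a set lifetime.
; Each hit spawns the hit Niagara effect and applies weapon damage, then destroys the projectile unless bouncing is enabled.
; A delay started at BeginPlay handles expiry, spawning a blue fire effect at the projectile's location before destroying it.
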(event `self.ReceiveBeginPlay`
  (`KismetSystemLibrary.Delay` (`self.Kys`))
  (`NiagaraFunctionLibrary.SpawnSystemAtLocation` "/Game/StudentWork/PlayerWeapion/VFX/NS_fireEffectBlue.NS_fireEffectBlue" (`self.K2_GetActorLocation`) (`SceneComponent.K2_GetComponentRotation` (`self.StaticMesh`)))
  (`self.K2_DestroyActor`))

(event `self.StaticMesh.OnComponentHit`
  (params (HitComponent :type "PrimitiveComponent Object Reference") (OtherActor :type "Actor Object Reference") (OtherComp :type "PrimitiveComponent Object Reference") (NormalImpulse :type "Vector Structure") (Hit :type "HitResult Structure (by ref)"))
  (bind _output_get (set `self.Other Actor_0` OtherActor))
  (`NiagaraFunctionLibrary.SpawnSystemAtLocation` (`self.HitVFX`) (`self.K2_GetActorLocation`))
  (`GameplayStatics.ApplyDamage` _output_get (`self.WeaponDMG`))
  (if (not (`self.ShouldBounce`))
    (`self.K2_DestroyActor`)))

(fn `UserConstructionScript`)