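; BP_RqailGunProjectile is a railgun projectile that deals radial damage when its static mesh hits something.
; BeginPlay sets the weapon damage and assigns a red Niagara hit effect, which this graph does not spawn itself.
; On hit it applies damage around the mesh location and draws a red debug sphere matching the blast radius.
; The construction script only calls its parent.
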(event `self.ReceiveBeginPlay`
  (set `self.WeaponDMG` 99.99)
  (set `self.HitVFX` "/Game/StudentWork/PlayerWeapion/VFX/NS_HitEffectRed.NS_HitEffectRed"))

(event `self.StaticMesh.OnComponentHit`
  (params (HitComponent :type "PrimitiveComponent Object Reference") (OtherActor :type "Actor Object Reference") (OtherComp :type "PrimitiveComponent Object Reference") (NormalImpulse :type "Vector Structure") (Hit :type "HitResult Structure (by ref)"))
  (bind _returnvalue (`SceneComponent.K2_GetComponentLocation` (`self.StaticMesh`)))
  (`GameplayStatics.ApplyRadialDamage` :`BaseDamage` (`self.WeaponDMG`) :`Origin` _returnvalue :`DamageRadius` 350.0 :`DamageCauser` self :`InstigatedByController` null)
  (`KismetSystemLibrary.DrawDebugSphere` _returnvalue 350.0 12 (struct :`R` 1.0 :`B` 0.025346 :`A` 1.0) 1.0 1.0))

(fn `UserConstructionScript`
  (`parent.UserConstructionScript`))