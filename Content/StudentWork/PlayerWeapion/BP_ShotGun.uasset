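; BP_ShotGun is a player shotgun weapon Blueprint that fires spreads of BP_ShotGunAmmo projectiles with a laser shot sound.
; Triggered checks a Cooldown flag, then loops SpawnProj several times with no delay between volleys, setting a one-second timer that clears the flag.
; Each SpawnProj spawns one projectile at each of eight Arrow components, using their world location and rotation to define the pattern.
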(event `Spawn Proj`
  ;[1 1 1] fire
  (`self.fire` (`self.Arrow1`))
  (`self.fire` (`self.Arrow2`))
  (`self.fire` (`self.Arrow3`))
  (`self.fire` (`self.Arrow4`))
  (`self.fire` (`self.Arrow5`))
  (`self.fire` (`self.Arrow6`))
  (`self.fire` (`self.Arrow7`))
  (`self.fire` (`self.Arrow8`)))

(event `fire`
  (params (Arrow :type "ArrowComponent Object Reference"))
  ;[1 1 1] spawnProj
  (`|SpawnActorFromClass` "/Game/StudentWork/PlayerWeapion/BP_ShotGunAmmo.BP_ShotGunAmmo_C" (`KismetMathLibrary.MakeTransform` (`SceneComponent.K2_GetComponentLocation` Arrow) (`SceneComponent.K2_GetComponentRotation` Arrow)) "Undefined" "MultiplyWithRoot" null null))

(event `self.Triggered`
  ;[1 1 1] attack speed
  (if (not (`self.Cooldown`))
    (for _ (range 3)
      (`self.Spawn Proj`)
      (`GameplayStatics.PlaySoundAtLocation` "/Game/StudentWork/sound/laser-shot-ingame-230500.laser-shot-ingame-230500" (`SceneComponent.GetSocketLocation` (`self.StaticMesh`) "None") (struct) 1.0 1.0 0.0 null null null null)
      (set `self.Cooldown` true)
      (`KismetSystemLibrary.K2_SetTimerDelegate` (delegate `End Cooldown`) 1.0))))

(event `End Cooldown`
  ;[1 1 1] attack speed
  (set `self.Cooldown` false))

(fn `UserConstructionScript`
  (`parent.UserConstructionScript`))