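; BP_RailGunWeapion is a tank railgun weapon that fires projectiles when triggered, rate-limited by an AttackSpeed cooldown timer.
; Each shot spawns the AmmoType actor at the Arrow and copies the tank's ExtraDMG onto it if it is a BP_Projectile.
; Successful shots also play a laser sound and red Niagara muzzle effect.
; A Timeline offsets the gun mesh along X for recoil, with a delayed transform reset.
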(event `self.Triggered`
  (if (not (`self.Cooldown`))
    (`self.SpawnProj`)
    (set `self.Cooldown` true)
    (`KismetSystemLibrary.K2_SetTimerDelegate` (delegate `End Cooldown`) (`self.AttackSpeed`))))

(event `End Cooldown`
  (set `self.Cooldown` false))

(event `SpawnProj`
  (bind _arrow (`self.Arrow`))
  (bind _returnvalue (`SceneComponent.K2_GetComponentLocation` _arrow))
  (bind _returnvalue_2 (`SceneComponent.K2_GetComponentRotation` _arrow))
  ;[1 1 1] SpawnProj
  (`self.Animtion`)
  (bind _returnvalue_3 (`|SpawnActorFromClass` (`self.Ammo Type`) (`KismetMathLibrary.MakeTransform` _returnvalue _returnvalue_2) "Undefined" "MultiplyWithRoot" null null))
  (bind _asbp_projectile (cast `/Game/StudentWork/PlayerWeapion/BP_Projectile` _returnvalue_3))
  (set `/Game/StudentWork/PlayerWeapion/BP_Projectile.Extra_DMG` (`/Game/Blueprints/BP_PlayerCharacter.Extra DMG` (`self.MyTank`)) _asbp_projectile)
  (`GameplayStatics.PlaySoundAtLocation` "/Game/StudentWork/sound/laser-shot-ingame-230500.laser-shot-ingame-230500" _returnvalue (struct) 1.0 1.0 0.0 null null null null)
  (`NiagaraFunctionLibrary.SpawnSystemAtLocation` "/Game/StudentWork/PlayerWeapion/VFX/NS_fireEffectRed.NS_fireEffectRed" _returnvalue _returnvalue_2))

(event `Animtion`
  (bind (_direction _newtrack_0) (`Timeline|Timeline`)
    (:`Update`
      (`SceneComponent.K2_SetRelativeTransform` (`self.RailGun_Cube_005`) (`KismetMathLibrary.MakeTransform` (`KismetMathLibrary.MakeVector` (* _newtrack_0 -30.0))) false false)
      (`KismetSystemLibrary.Delay` 0.1)
      (`SceneComponent.K2_SetRelativeTransform` (`self.RailGun_Cube_005`) (`KismetMathLibrary.MakeTransform` (0.0 0.0 0.0)) false false))))

(fn `UserConstructionScript`
  (`parent.UserConstructionScript`))