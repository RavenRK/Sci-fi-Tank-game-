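; Twin-barrel machine gun weapon that fires blue-effect laser shots when triggered, rate-limited by an AttackSpeed cooldown timer.
; Each shot pair spawns BP_Projectile at two arrow components, with a laser sound and Niagara fire effect at each.
; The first barrel's spawn event also plays a timeline recoil that offsets the gun mesh along X, then resets its transform after a short delay.
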(event `Animtion`
  ;[1 1 1] animtion
  (bind (_direction _newtrack_0) (`Timeline|Timeline`)
    (:`Update`
      (`SceneComponent.K2_SetRelativeTransform` (`self.machenGun_Cube_004`) (`KismetMathLibrary.MakeTransform` (`KismetMathLibrary.MakeVector` (* _newtrack_0 -25.0))) false false)
      (`KismetSystemLibrary.Delay` 0.1)
      (`SceneComponent.K2_SetRelativeTransform` (`self.machenGun_Cube_004`) (`KismetMathLibrary.MakeTransform` (0.0 0.0 0.0)) false false))))

(event `self.Triggered`
  ;[1 1 1] Main
  (if (not (`self.Cooldown`))
    (`self.SpawnProj_1`)
    (`self.SpawnProj_2`)
    (set `self.Cooldown` true)
    (`KismetSystemLibrary.K2_SetTimerDelegate` (delegate `End Cooldown`) (`self.AttackSpeed`))))

(event `End Cooldown`
  ;[1 1 1] Main
  (set `self.Cooldown` false))

(event `SpawnProj_1`
  (bind _arrow (`self.Arrow`))
  (bind _returnvalue (`SceneComponent.K2_GetComponentLocation` _arrow))
  (bind _returnvalue_2 (`SceneComponent.K2_GetComponentRotation` _arrow))
  ;[1 1 1] Spawn Proj play sound and spawn fire effect
  (`|SpawnActorFromClass` "/Game/StudentWork/PlayerWeapion/BP_Projectile.BP_Projectile_C" (`KismetMathLibrary.MakeTransform` _returnvalue _returnvalue_2) "Undefined" "MultiplyWithRoot" null null)
  (`GameplayStatics.PlaySoundAtLocation` "/Game/StudentWork/sound/laser-shot-ingame-230500.laser-shot-ingame-230500" _returnvalue (struct) 1.0 1.0 0.0 null null null null)
  (`NiagaraFunctionLibrary.SpawnSystemAtLocation` "/Game/StudentWork/PlayerWeapion/VFX/NS_fireEffectBlue.NS_fireEffectBlue" _returnvalue _returnvalue_2)
  (`self.Animtion`))

(event `SpawnProj_2`
  (bind _arrow1 (`self.Arrow1`))
  (bind _returnvalue (`SceneComponent.K2_GetComponentLocation` _arrow1))
  (bind _returnvalue_2 (`SceneComponent.K2_GetComponentRotation` _arrow1))
  ;[1 1 1] Spawn Proj play sound and spawn fire effect
  (`|SpawnActorFromClass` "/Game/StudentWork/PlayerWeapion/BP_Projectile.BP_Projectile_C" (`KismetMathLibrary.MakeTransform` _returnvalue _returnvalue_2) "Undefined" "MultiplyWithRoot" null null)
  (`GameplayStatics.PlaySoundAtLocation` "/Game/StudentWork/sound/laser-shot-ingame-230500.laser-shot-ingame-230500" _returnvalue (struct) 1.0 1.0 0.0 null null null null)
  (`NiagaraFunctionLibrary.SpawnSystemAtLocation` "/Game/StudentWork/PlayerWeapion/VFX/NS_fireEffectBlue.NS_fireEffectBlue" _returnvalue _returnvalue_2))

(fn `UserConstructionScript`
  (`parent.UserConstructionScript`))