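; Flamethrower weapon for the player's tank that damages whatever is caught in a short line ahead of it.
; Each trigger activates the Niagara effect and, when off cooldown, fires SpawnProj, which runs a forward multi-sphere trace from the Arrow instead of spawning a projectile.
; Every hit takes weapon damage scaled by the tank's ExtraDMG.
; An AttackSpeed timer clears the cooldown and re-activates Niagara with a reset.
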(event `self.Triggered`
  ;[1 1 1] Trigger fire
  (`ActorComponent.Activate` (`self.Niagara`) false)
  (if (not (`self.Cooldown`))
    (`self.SpawnProj`)
    (set `self.Cooldown` true)
    (`KismetSystemLibrary.K2_SetTimerDelegate` (delegate `CustomEvent`) (`self.AttackSpeed`))))

(event `CustomEvent`
  ;[1 1 1] Trigger fire
  (set `self.Cooldown` false)
  (`ActorComponent.Activate` (`self.Niagara`) true))

(event `self.SpawnProj`
  (bind _arrow (`self.Arrow`))
  (bind _returnvalue_location (`KismetMathLibrary.BreakTransform` (`SceneComponent.K2_GetComponentToWorld` _arrow)))
  ;[1 1 1] SpawnPorJ
  (bind _outhits (`KismetSystemLibrary.SphereTraceMultiForObjects` _returnvalue_location (+ _returnvalue_location (* (`SceneComponent.GetForwardVector` _arrow) 600.0)) 65.0 (`self.Object Types`)))
  (for _array_element _outhits
    (`GameplayStatics.ApplyDamage` (`.HitActor` (`GameplayStatics.BreakHitResult` _array_element)) (* (`self.WeaponDMG`) (`/Game/Blueprints/BP_PlayerCharacter.Extra DMG` (`self.MyTank`))))))

(fn `UserConstructionScript`
  (`parent.UserConstructionScript`))